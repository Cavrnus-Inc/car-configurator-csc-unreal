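; Animated passenger car door that opens and closes on click, with its state shared through a Space connection.
; On BeginPlay it awaits a connection and binds to the boolean PassengerDoorAnimation property in the Car container.
; Clicking the ClickBox posts the toggled value rather than moving the door directly.
; The property update then plays or reverses an eased timeline that sets the root's world yaw.
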(event `self.ReceiveBeginPlay`
  (`CavrnusFunctionLibrary.AwaitAnySpaceConnection` (delegate `SpaceConnected_Passenger`)))

(event `SpaceConnected_Passenger`
  (params (SpaceConnection :type "CavrnusSpaceConnection Structure"))
  (bind _output_get (set `self.ConnectedSpace` SpaceConnection))
  (`CavrnusFunctionLibrary.BindBooleanPropertyValue` _output_get "Car" "PassengerDoorAnimation" (delegate `OpenPassengerDoor`)))

(event `OpenPassengerDoor`
  (params (Value :type Boolean) (ContainerName :type String) (PropertyName :type String))
  ;[1 1 1] Open Car Door - True is Closed, False is Open
  (bind _output_get (set `self.IsClosed?` Value))
  (if _output_get
    (bind (_direction _easeopen) (`Timeline|Passenger_Animation` :!label _label)
      (:`Update`
        (`SceneComponent.K2_SetWorldRotation` (`self.DefaultSceneRoot`) (`KismetMathLibrary.MakeRotator` 0.0 0.0 _easeopen) false false)))
    (else
      (goto _label :!via `Reverse`))))

(event `self.ClickBox.OnClicked`
  (params (TouchedComponent :type "PrimitiveComponent Object Reference") (ButtonPressed :type "Key Structure"))
  (bind _output_get (set `self.IsClosed?` (not (`self.IsClosed?`))))
  (`CavrnusFunctionLibrary.PostBoolPropertyUpdate` (`self.ConnectedSpace`) "Car" "PassengerDoorAnimation" _output_get))

(fn `UserConstructionScript`)