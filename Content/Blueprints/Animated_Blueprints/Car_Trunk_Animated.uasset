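; Animated car trunk Blueprint that opens and closes on click, with its state shared through a space connection.
; On BeginPlay it awaits a space connection, then binds to the "TrunkAnimation" boolean in the "Car" container.
; Clicking the ClickBox flips IsClosed and posts it to that property.
; Property updates play or reverse a timeline that rotates the root in world space (true is closed), via handlers still named for the driver door.
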(event `self.ReceiveBeginPlay`
  (`CavrnusFunctionLibrary.AwaitAnySpaceConnection` (delegate `SpaceConnected-Driver`)))

(event `SpaceConnected-Driver`
  (params (SpaceConnection :type "CavrnusSpaceConnection Structure"))
  (bind _output_get (set `self.ConnectedSpace` SpaceConnection))
  (`CavrnusFunctionLibrary.BindBooleanPropertyValue` _output_get "Car" "TrunkAnimation" (delegate `OpenDriverDoor`)))

(event `OpenDriverDoor`
  (params (Value :type Boolean) (ContainerName :type String) (PropertyName :type String))
  ;[1 1 1] Open Car Door - True is Closed, False is Open
  (if Value
    (bind (_direction _easeopen) (`Timeline|Trunk_Timeline` :!via `Reverse` :!label _label)
      (:`Update`
        (`SceneComponent.K2_SetWorldRotation` (`self.DefaultSceneRoot`) (`KismetMathLibrary.MakeRotator` 0.0 _easeopen) false false)))
    (else
      (goto _label))))

(event `self.ClickBox.OnClicked`
  (params (TouchedComponent :type "PrimitiveComponent Object Reference") (ButtonPressed :type "Key Structure"))
  (bind _output_get (set `self.IsClosed?` (not (`self.IsClosed?`))))
  (`CavrnusFunctionLibrary.PostBoolPropertyUpdate` (`self.ConnectedSpace`) "Car" "TrunkAnimation" _output_get))

(fn `UserConstructionScript`)