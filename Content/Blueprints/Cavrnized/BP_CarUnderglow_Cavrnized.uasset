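; Car underglow actor whose visibility follows a shared boolean property in a Cavrnus space.
; On BeginPlay it waits for a space connection, then binds to the "UnderGlowVis" property in the "Car" container.
; Each update shows or hides the whole actor and refreshes the underglow toggle button color on the first WB_CarConfigCavrnized widget found.
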(event `self.ReceiveBeginPlay`
  (`CavrnusFunctionLibrary.AwaitAnySpaceConnection` (delegate `SetSpaceConnection`)))

(event `SetSpaceConnection`
  (params (SpaceConnection :type "CavrnusSpaceConnection Structure"))
  (bind _output_get (set `self.ConnectedSpace` SpaceConnection))
  (`CavrnusFunctionLibrary.BindBooleanPropertyValue` _output_get "Car" "UnderGlowVis" (delegate `UpdateUnderglowLight`)))

(event `UpdateUnderglowLight`
  (params (Value :type Boolean) (ContainerName :type String) (PropertyName :type String))
  ;[1 1 1] Toggle Underglow Light
  (bind _output_get (set `self.UnderglowOn?` Value))
  (bind _foundwidgets (`WidgetBlueprintLibrary.GetAllWidgetsOfClass` "/Game/UI/WB_CarConfigCavrnized.WB_CarConfigCavrnized_C" false))
  (bind _output (`|GetArrayItem` _foundwidgets))
  (`/Game/UI/WB_CarConfigCavrnized.ToggleUnderglowBTNColor` _output (`/Game/UI/WB_CarConfigCavrnized.BTN_StatelyToggleUnderglow` _output))
  (`self.SetActorHiddenInGame` (not _output_get)))

(fn `UserConstructionScript`)