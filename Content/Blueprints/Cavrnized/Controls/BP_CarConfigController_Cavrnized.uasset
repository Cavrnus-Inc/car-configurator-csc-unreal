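; Car configurator controller that sets up a shared, synced paint material on BeginPlay.
; It creates a dynamic instance from its own mesh's first material and hands it to the SyncMaterial component.
; Each SyncMaterialTextureParam child of that component receives the CarTextureMap.
; Inside that same child loop, the instance is applied to slot 0 of every StaticMeshActor tagged CarPaint, so all painted parts share one material.
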(event `self.ReceiveBeginPlay`
  (bind _staticmeshcomponent (`self.StaticMeshComponent`))
  (bind _syncmaterial (`self.SyncMaterial`))
  (bind _returnvalue (`PrimitiveComponent.CreateDynamicMaterialInstance` _staticmeshcomponent 0 (`PrimitiveComponent.GetMaterial` _staticmeshcomponent 0) "MID_CarColor"))
  (`CavrnusSyncMaterial.SetMaterialInstance` _syncmaterial _returnvalue)
  (for _array_element (`SceneComponent.GetChildrenComponents` _syncmaterial true)
    (bind _assync_material_texture_param (cast `/CavrnusConnector/SampleBehaviors/SyncMaterialTextureParam` _array_element))
    (set `/CavrnusConnector/SampleBehaviors/SyncMaterialTextureParam.TextureMap` (`self.CarTextureMap`) _assync_material_texture_param)
    (bind _outactors (`GameplayStatics.GetAllActorsOfClassWithTag` "/Script/Engine.StaticMeshActor" "CarPaint"))
    (for _array_element_2 _outactors
      (`PrimitiveComponent.SetMaterial` (`StaticMeshActor.StaticMeshComponent` _array_element_2) 0 _returnvalue))))

(fn `UserConstructionScript`)