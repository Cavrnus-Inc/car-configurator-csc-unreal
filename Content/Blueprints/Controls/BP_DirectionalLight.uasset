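; Directional light actor whose sun yaw and shadow amount are synced through a Cavrnus space as float properties on the "Car" container.
; Once connected, it binds both properties, applying updates to the root's rotation and the light's shadow amount.
; Setter events either stream transient updates, reusing a live updater, or post committed values.
; Separate events finalize each transient; EndPlay finalizes only the light direction.
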(event `self.ReceiveBeginPlay`
  ;[1 1 1] Phase 1: Connect to the Space
  (set `self.SunAngleParameterName` "SunRotation")
  (set `self.ShadowStrengthParamName` "ShadowStrength")
  ;;[1 1 1] Wait for Cavrnus to Connect
  (`CavrnusFunctionLibrary.AwaitAnySpaceConnection` (delegate `SetSpaceConnection`)))

(event `SetSpaceConnection`
  (params (SpaceConnection :type "CavrnusSpaceConnection Structure"))
  ;[1 1 1] Phase 1: Connect to the Space
  (set `self.ConnectedSpace` SpaceConnection)
  (`|ExecutionSequence`
    (:`then_0`
      (`self.BindSunAngleProperty`))
    (:`then_1`
      (`self.BindShadowAmount`))))

(event `BindSunAngleProperty`
  ;[1 1 1] PHASE 2: Bind Properties to Receive Updates from Journal
  ;;[1 1 1] Bind Sun Angle Property
  ;;;[1 1 1] Wait for Sun Angle Property Change
  (`CavrnusFunctionLibrary.BindFloatPropertyValue` (`self.ConnectedSpace`) "Car" (`self.SunAngleParameterName`) (delegate `UpdateDirectionLightWorldRotation`)))

(event `BindShadowAmount`
  ;[1 1 1] PHASE 2: Bind Properties to Receive Updates from Journal
  ;;[1 1 1] Bind Shadow Amount Property
  ;;;[1 1 1] Wait for Property Change
  (`CavrnusFunctionLibrary.BindFloatPropertyValue` (`self.ConnectedSpace`) "Car" (`self.ShadowStrengthParamName`) (delegate `UpdateShadowStrength`)))

(event `UpdateDirectionLightWorldRotation`
  (params (Value :type "Float (single-precision)") (ContainerName :type String) (PropertyName :type String))
  (bind _defaultsceneroot (`self.DefaultSceneRoot`))
  (bind (_returnvalue_roll _returnvalue_pitch) (`KismetMathLibrary.BreakRotator` (`SceneComponent.K2_GetComponentRotation` _defaultsceneroot)))
  ;[1 1 1] PHASE 2: Bind Properties to Receive Updates from Journal
  ;;[1 1 1] Bind Sun Angle Property
  (bind _result (`/Engine/EditorBlueprintResources/StandardMacros.NegateFloat` (- Value 0.0))
    (:`  `
      ;;;[1 1 1] Set World Rotation from Property Change
      (`SceneComponent.K2_SetWorldRotation` _defaultsceneroot (`KismetMathLibrary.MakeRotator` _returnvalue_roll _returnvalue_pitch _result) false false))))

(event `UpdateShadowStrength`
  (params (Value :type "Float (single-precision)") (ContainerName :type String) (PropertyName :type String))
  ;[1 1 1] PHASE 2: Bind Properties to Receive Updates from Journal
  ;;[1 1 1] Bind Shadow Amount Property
  ;;;[1 1 1] Set Shadow Amount from Property Change
  (`DirectionalLightComponent.SetShadowAmount` (`self.DirectionalLight`) Value))

(event `SetLightDirectionTransient`
  (params (`IsTransient?` :type Boolean))
  (bind _connectedspace (`self.ConnectedSpace`))
  (bind _transientdirectionallight (`self.TransientDirectionalLight`))
  ;[1 1 1] Phase 3: Update the Journal directly by Posting Transient Values
  ;;[1 1 1] Post DirectionalLight to the Journal as Transient
  (set `self.IsTransient` `IsTransient?`)
  (bind _returnvalue (`CavrnusFunctionLibrary.IsConnectedToAnySpace` :!label _label))
  (if _returnvalue
    (if (`self.IsTransient`)
      (`/Engine/EditorBlueprintResources/StandardMacros.IsValid` _transientdirectionallight
        (:`Is Valid`
          (`CavrnusLiveFloatPropertyUpdate.UpdateWithNewData` _transientdirectionallight (stale `SetLightDirection` LightAngleDegrees)))
        (:`Is Not Valid`
          (bind _returnvalue_2 (`CavrnusFunctionLibrary.BeginTransientFloatPropertyUpdate` _connectedspace "Car" (`self.SunAngleParameterName`) (stale `SetLightDirection` LightAngleDegrees)))
          (set `self.TransientDirectionalLight` _returnvalue_2)))
      (else
        ;;;[1 1 1] Commit Property
        (`CavrnusFunctionLibrary.PostFloatPropertyUpdate` _connectedspace "Car" (`self.SunAngleParameterName`) (stale `SetLightDirection` LightAngleDegrees))))))

(event `SetShadowAmountTransient`
  (params (`IsTransient?` :type Boolean))
  (bind _connectedspace (`self.ConnectedSpace`))
  (bind _transientshadowamount (`self.TransientShadowAmount`))
  ;[1 1 1] Phase 3: Update the Journal directly by Posting Transient Values
  ;;[1 1 1] Post Shadow Amount to the Journal as Transient
  (set `self.IsTransient` `IsTransient?`)
  (bind _returnvalue (`CavrnusFunctionLibrary.IsConnectedToAnySpace` :!label _label_2))
  (if _returnvalue
    (if (`self.IsTransient`)
      (`/Engine/EditorBlueprintResources/StandardMacros.IsValid` _transientshadowamount
        (:`Is Valid`
          (`CavrnusLiveFloatPropertyUpdate.UpdateWithNewData` _transientshadowamount (stale `SetShadowAmount` NewShadowAmount)))
        (:`Is Not Valid`
          (bind _returnvalue_2 (`CavrnusFunctionLibrary.BeginTransientFloatPropertyUpdate` _connectedspace "Car" (`self.ShadowStrengthParamName`) (stale `SetShadowAmount` NewShadowAmount)))
          (set `self.TransientShadowAmount` _returnvalue_2)))
      (else
        ;;;[1 1 1] Commit Property
        (`CavrnusFunctionLibrary.PostFloatPropertyUpdate` _connectedspace "Car" (`self.ShadowStrengthParamName`) (stale `SetShadowAmount` NewShadowAmount))))))

(event `SetLightDirection`
  (params (LightAngleDegrees :type "Float (double-precision)"))
  ;[1 1 1] Phase 3: Update the Journal directly by Posting Transient Values
  ;;[1 1 1] Post DirectionalLight to the Journal as Transient
  (goto _label))

(event `SetShadowAmount`
  (params (NewShadowAmount :type "Float (double-precision)"))
  ;[1 1 1] Phase 3: Update the Journal directly by Posting Transient Values
  ;;[1 1 1] Post Shadow Amount to the Journal as Transient
  (goto _label_2))

(event `FinalizeDirectionalLight`
  (bind _transientdirectionallight (`self.TransientDirectionalLight`))
  ;[1 1 1] Phase 4: Finalize Directional Light Property in Journal
  (if (`KismetSystemLibrary.IsValid` _transientdirectionallight)
    (`CavrnusLiveFloatPropertyUpdate.Finalize` _transientdirectionallight (`.Z` (`KismetMathLibrary.BreakVector3f` (`.Z` (`KismetMathLibrary.BreakRotIntoAxes` (`SceneComponent.K2_GetComponentRotation` (`self.DirectionalLight`)))))))))

(event `FinalizeShadowAmount`
  (bind _transientshadowamount (`self.TransientShadowAmount`))
  ;[1 1 1] Phase 4: Finalize Shadow Amount Property in Journal
  (if (`KismetSystemLibrary.IsValid` _transientshadowamount)
    (`CavrnusLiveFloatPropertyUpdate.Finalize` _transientshadowamount (`DirectionalLightComponent.ShadowAmount` (`self.DirectionalLight`)))))

(event `self.ReceiveEndPlay`
  (params (EndPlayReason :type "EEndPlayReason Enum" :default "Destroyed"))
  ;[1 1 1] Phase 4: Finalize On Exit Space
  (bind _returnvalue (`CavrnusFunctionLibrary.IsConnectedToAnySpace`))
  (if _returnvalue
    (`self.FinalizeDirectionalLight`)))

(fn `UserConstructionScript`)