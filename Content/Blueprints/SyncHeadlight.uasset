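; SyncHeadlight exposes the car's headlights as a single boolean property that can be read and set.
; On BeginPlay it caches every SpotLight actor tagged "Headlights".
; SetBoolean shows or hides all cached lights, then blocks further writes for a fraction of a second through a UseProperties flag that a timer re-enables.
; GetBoolean reports the state from the first light's visibility.
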(event `self.ReceiveBeginPlay`
  (bind _outactors (`GameplayStatics.GetAllActorsOfClassWithTag` "/Script/Engine.SpotLight" "Headlights"))
  (set `self.CarLights` _outactors))

(event `self.SetBoolean`
  (params (bPropertyValue :type Boolean))
  (if (`self.UseProperties`)
    (for _array_element (`self.CarLights`)
      (`Actor.SetActorHiddenInGame` _array_element (not bPropertyValue))
      (set `self.UseProperties` false)
      (`KismetSystemLibrary.K2_SetTimerDelegate` (delegate `PassToNext`) 0.1))))

(event `PassToNext`
  (set `self.UseProperties` true))

(fn `GetBoolean`
  (returns (ReturnValue :type Boolean))
  (return (not (`Actor.bHidden` (`|GetArrayItem` (`self.CarLights`))))))