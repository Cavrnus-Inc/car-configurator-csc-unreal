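; SyncLightColor is a color sync component that exposes a parent spot light's color through GetColor and SetColor.
; On BeginPlay it caches its first parent component as the light, printing a warning if that is not a SpotLightComponent.
; SetColor applies the incoming property value, then finds the first WB_CarConfigCavrnized widget and calls its underglow button color toggle, coupling it to that car configurator UI.
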(event `self.ReceiveBeginPlay`
  (bind _asspot_light_component (cast `SpotLightComponent` (`|GetArrayItem` (`self.GetParentComponents`)))
    (:`then`
      (set `self.Light` _asspot_light_component))
    (:`CastFailed`
      (`KismetSystemLibrary.PrintString` "SyncColor must exist below a Light Component."))))

(event `self.SetColor`
  (params (PropertyValue :type "LinearColor Structure"))
  (bind _asspot_light_component (cast `SpotLightComponent` (`self.Light`)))
  (`LightComponent.SetLightColor` _asspot_light_component PropertyValue true)
  (bind _foundwidgets (`WidgetBlueprintLibrary.GetAllWidgetsOfClass` "/Game/Widgets/WB_CarConfigCavrnized.WB_CarConfigCavrnized_C" false))
  (bind _output (`|GetArrayItem` _foundwidgets))
  (`/Game/Widgets/WB_CarConfigCavrnized.ToggleUnderglowBTNColor` _output (`/Game/Widgets/WB_CarConfigCavrnized.BTN_StatelyToggleUnderglow` _output)))

(fn `GetColor`
  (returns (ReturnValue :type "LinearColor Structure"))
  (return (`LightComponentBase.GetLightColor` (`self.Light`))))