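; SyncUnderglow exposes the visibility of an underglow spotlight as a boolean property.
; BeginPlay caches the first SpotLight actor tagged "Underglow", and GetBoolean reports whether it is visible.
; SetBoolean shows or hides the light only while UseProperties is true, then clears that flag and re-arms it by timer half a second later, throttling rapid changes.
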(event `self.ReceiveBeginPlay`
  (bind _outactors (`GameplayStatics.GetAllActorsOfClassWithTag` "/Script/Engine.SpotLight" "Underglow"))
  (set `self.UnderglowLight` (`|GetArrayItem` _outactors)))

(event `self.SetBoolean`
  (params (bPropertyValue :type Boolean))
  (if (`self.UseProperties`)
    (`Actor.SetActorHiddenInGame` (`self.UnderglowLight`) (not bPropertyValue))
    (set `self.UseProperties` false)
    (`KismetSystemLibrary.K2_SetTimerDelegate` (delegate `PassToNext`) 0.5)))

(event `PassToNext`
  (set `self.UseProperties` true))

(fn `GetBoolean`
  (returns (ReturnValue :type Boolean))
  (return (not (`Actor.bHidden` (`self.UnderglowLight`)))))